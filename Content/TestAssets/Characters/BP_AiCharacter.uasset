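; BP_AiCharacter is an AI character Blueprint with switchable jog and walk animation and a target-seeking direction helper.
; Two custom events swap the mesh's Animation Blueprint between jog and walk, disabling controller-yaw rotation for jog and enabling it for walk.
; GetDesiredVelocity returns a unit direction toward TargetLocation while it is beyond Reach, otherwise a zero vector, and updates IsMoving as a side effect.
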(event `ChangeAnimBPTo_Jog`
  (bind _mesh (`self.Mesh`))
  (`SkeletalMeshComponent.SetAnimationMode` _mesh "AnimationBlueprint")
  (`SkeletalMeshComponent.SetAnimInstanceClass` _mesh "/Game/TestAssets/Animations/ABP_AI_Jog.ABP_AI_Jog_C")
  (set `self.bUseControllerRotationYaw` false))

(event `ChangeAnimBPTo_Walk`
  (bind _mesh (`self.Mesh`))
  (`SkeletalMeshComponent.SetAnimationMode` _mesh "AnimationBlueprint")
  (`SkeletalMeshComponent.SetAnimInstanceClass` _mesh "/Game/TestAssets/Animations/ABP_AI_Walk.ABP_AI_Walk_C")
  (set `self.bUseControllerRotationYaw` true))

(fn `GetDesiredVelocity`
  (returns (DesiredVelocity :type "Vector Structure"))
  (bind _returnvalue (`self.K2_GetActorLocation`))
  (bind _target_location (`self.Target location`))
  (if (> (`KismetMathLibrary.Vector_Distance` _target_location _returnvalue) (`self.Reach`))
    (set `self.IsMoving` true)
    (return (`KismetMathLibrary.GetDirectionUnitVector` _returnvalue _target_location))
    (else
      (set `self.IsMoving` false)
      (return (0.0 0.0 0.0)))))

(fn `UserConstructionScript`)